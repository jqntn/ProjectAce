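; Showcase Blueprint for the West B2 bomber that exposes its moving parts and appearance to generic checkbox, slider and twin-slider controls.
; Each control event forwards its value to aircraft functions for damage display, elevons, rudders, light emissivity, bomb hatches, engine covers and landing gear.
; Gear retraction and suspension are mutually exclusive: adjusting one resets the other to zero.
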(event `/Game/VigilanteContent/Shared/Blueprints/Showcase/Interfaces/BP_ShowcaseControlsInterface.SetCheckboxVariable0`
  (params (NewState :type Boolean))
  (`self.SetShowDamaged` NewState))

(event `/Game/VigilanteContent/Shared/Blueprints/Showcase/Interfaces/BP_ShowcaseControlsInterface.SetSliderVariable0`
  (params (NewValue :type "Float (single-precision)"))
  (`self.SetInboardEvelons` NewValue))

(event `/Game/VigilanteContent/Shared/Blueprints/Showcase/Interfaces/BP_ShowcaseControlsInterface.SetSliderVariable1`
  (params (NewValue :type "Float (single-precision)"))
  (`self.SetMidEvelons` NewValue))

(event `/Game/VigilanteContent/Shared/Blueprints/Showcase/Interfaces/BP_ShowcaseControlsInterface.SetSliderVariable2`
  (params (NewValue :type "Float (single-precision)"))
  (`self.SetOutboardEvelons` NewValue))

(event `/Game/VigilanteContent/Shared/Blueprints/Showcase/Interfaces/BP_ShowcaseControlsInterface.SetSliderVariable3`
  (params (NewValue :type "Float (single-precision)"))
  (`self.SetLightsEmissivity` NewValue))

(event `/Game/VigilanteContent/Shared/Blueprints/Showcase/Interfaces/BP_ShowcaseControlsInterface.SetTwinSliderVariable0`
  (params (`bFirstSlider?` :type Boolean) (NewFirstValue :type "Float (single-precision)") (NewSecondValue :type "Float (single-precision)"))
  (`self.RetractFrontWheel` NewFirstValue)
  (`self.RetractRearRWheel` NewSecondValue)
  (`self.RetractRearLWheel` NewSecondValue)
  (`self.SetFrontWheelSuspension` 0.0)
  (`self.SetRearWheelLSuspension` 0.0)
  (`self.SetRearWheelRSuspension` 0.0))

(event `/Game/VigilanteContent/Shared/Blueprints/Showcase/Interfaces/BP_ShowcaseControlsInterface.SetTwinSliderVariable1`
  (params (`bFirstSlider?` :type Boolean) (NewFirstValue :type "Float (single-precision)") (NewSecondValue :type "Float (single-precision)"))
  (`self.SetBombHatchRight` NewFirstValue)
  (`self.SetBombHatchLeft` NewSecondValue))

(event `/Game/VigilanteContent/Shared/Blueprints/Showcase/Interfaces/BP_ShowcaseControlsInterface.SetTwinSliderVariable2`
  (params (`bFirstSlider?` :type Boolean) (NewFirstValue :type "Float (single-precision)") (NewSecondValue :type "Float (single-precision)"))
  (`self.SetFrontWheelSuspension` NewFirstValue)
  (`self.SetRearWheelLSuspension` NewSecondValue)
  (`self.SetRearWheelRSuspension` NewSecondValue)
  (`self.RetractFrontWheel` 0.0)
  (`self.RetractRearRWheel` 0.0)
  (`self.RetractRearLWheel` 0.0))

(event `/Game/VigilanteContent/Shared/Blueprints/Showcase/Interfaces/BP_ShowcaseControlsInterface.SetTwinSliderVariable3`
  (params (`bFirstSlider?` :type Boolean) (NewFirstValue :type "Float (single-precision)") (NewSecondValue :type "Float (single-precision)"))
  (`self.SetRudderLeftWing` NewFirstValue)
  (`self.SetRudderRightWing` NewSecondValue))

(event `/Game/VigilanteContent/Shared/Blueprints/Showcase/Interfaces/BP_ShowcaseControlsInterface.SetTwinSliderVariable4`
  (params (`bFirstSlider?` :type Boolean) (NewFirstValue :type "Float (single-precision)") (NewSecondValue :type "Float (single-precision)"))
  (`self.OpenEngineCoverRight1` NewFirstValue)
  (`self.OpenEngineCoverRight2` NewFirstValue)
  (`self.OpenEngineCoverLeft1` NewSecondValue)
  (`self.OpenEngineCoverLeft2` NewSecondValue))

(fn `UserConstructionScript`
  (`parent.UserConstructionScript`))